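; BP_CannonMp5 is an aimable cannon that fires a physics BP_Object1 projectile at an adjustable speed.
; RotateUp and RotateDown step the roll of the mesh and BulletREF muzzle point; their pitch and yaw captures are unconnected.
; Released spawns the projectile at BulletREF and launches it along the actor-to-muzzle direction, which PredictingPath also uses to debug-draw the trajectory.
; AddSpeed raises launch speed, while ReduceSpeed reports a decrease but subtracts zero.
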(event `self.ReceiveBeginPlay`
  (bind (_returnvalue_roll _returnvalue_pitch _returnvalue_yaw) (`KismetMathLibrary.BreakRotator` (`SceneComponent.K2_GetComponentRotation` (`self.BulletREF`))))
  (bind (_returnvalue_roll_2 _returnvalue_pitch_2 _returnvalue_yaw_2) (`KismetMathLibrary.BreakRotator` (`SceneComponent.K2_GetComponentRotation` (`self.StaticMesh`))))
  (set `self.ArrowRotation` _returnvalue_roll)
  (set `self.CannonRotation` _returnvalue_roll_2))

(event `Rotate Up`
  (`GameplayStatics.PlaySound2D` "/Game/Lessons/Lesson5/miniProject5/National_University_of_Singapore__2_.National_University_of_Singapore__2_" 1.0 1.0 0.0 null null)
  (bind _output_get (set `self.ArrowRotation` (+ (`self.ArrowRotation`) 5.0)))
  (`SceneComponent.K2_SetWorldRotation` (`self.BulletREF`) (`KismetMathLibrary.MakeRotator` _output_get (`self.ArrowX`) (`self.ArrowZ`)) false false)
  (bind _output_get_2 (set `self.CannonRotation` (+ (`self.CannonRotation`) 5.0)))
  (`SceneComponent.K2_SetWorldRotation` (`self.StaticMesh`) (`KismetMathLibrary.MakeRotator` _output_get_2 (`self.CannonY`) (`self.CannonZ`)) false false))

(event `Rotate Down`
  (`GameplayStatics.PlaySound2D` "/Game/Lessons/Lesson5/miniProject5/National_University_of_Singapore__2_.National_University_of_Singapore__2_" 1.0 1.0 0.0 null null)
  (bind _output_get (set `self.ArrowRotation` (- (`self.ArrowRotation`) 5.0)))
  (`SceneComponent.K2_SetWorldRotation` (`self.BulletREF`) (`KismetMathLibrary.MakeRotator` _output_get (`self.ArrowX`) (`self.ArrowZ`)) false false)
  (bind _output_get_2 (set `self.CannonRotation` (- (`self.CannonRotation`) 5.0)))
  (`SceneComponent.K2_SetWorldRotation` (`self.StaticMesh`) (`KismetMathLibrary.MakeRotator` _output_get_2 (`self.CannonY`) (`self.CannonZ`)) false false))

(event `Add Speed`
  (`KismetSystemLibrary.PrintString` "Speed Increased by 100!")
  (set `self.Speed` (+ (`self.Speed`) 100.0)))

(event `Reduce Speed`
  (`KismetSystemLibrary.PrintString` "Speed reduced by 100!")
  (set `self.Speed` (- (`self.Speed`) 0.0)))

(event `Released`
  (bind _returnvalue (`|SpawnActorFromClass` "/Game/Lessons/Lesson5/miniProject5/BP_Object1.BP_Object1_C" (`KismetMathLibrary.MakeTransform` (`SceneComponent.K2_GetComponentLocation` (`self.BulletREF`)) (`self.K2_GetActorRotation`)) "Undefined" "MultiplyWithRoot" null null))
  (`PrimitiveComponent.SetPhysicsLinearVelocity` (`/Game/Lessons/Lesson5/miniProject5/BP_Object1.Throwable Object 1` _returnvalue) (* (`KismetMathLibrary.GetDirectionUnitVector` (`self.K2_GetActorLocation`) (`self.K2_GetActorLocation` _returnvalue)) (`self.Speed`)) false "None")
  (`GameplayStatics.PlaySound2D` "/Game/Lessons/Lesson5/miniProject5/cannon-shot-14799.cannon-shot-14799" 1.0 1.0 0.0 null null))

(event `Predicting Path`
  (bind _returnvalue (`SceneComponent.K2_GetComponentLocation` (`self.BulletREF`)))
  (`GameplayStatics.Blueprint_PredictProjectilePath_Advanced` (make `PredictProjectilePathParams` _returnvalue (* (`KismetMathLibrary.GetDirectionUnitVector` (`self.K2_GetActorLocation`) _returnvalue) (`self.Speed`)) false 0.0 3.0 true "ECC_WorldStatic" _ _ 100.0 0.0 "ForDuration")))

(fn `Interactable`
  (returns (Interactable :type Boolean))
  (return false))

(fn `UserConstructionScript`)