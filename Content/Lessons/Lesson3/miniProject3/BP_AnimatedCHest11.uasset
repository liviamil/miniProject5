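; BP_AnimatedCHest11 is an interactable chest actor with an animated lid.
; The LidRotation timeline starts on BeginPlay and drives the ChestLid's relative roll on each update while IsHit is false.
; Interact toggles IsHit: setting it true suspends lid updates, and clearing it calls Play on the timeline again, with no reverse path.
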(event `Interact`
  (if (`self.isHit`)
    (set `self.isHit` false)
    (bind (_direction _timeline) (`Timeline|LidRotation` :!label _label)
      (:`Update`
        (if (not (`self.isHit`))
          (`SceneComponent.K2_SetRelativeRotation` (`self.ChestLid`) (`KismetMathLibrary.MakeRotator` _timeline) false false))))
    (else
      (set `self.isHit` true))))

(event `self.ReceiveBeginPlay`
  (goto _label))

(fn `UserConstructionScript`)