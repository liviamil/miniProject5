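; Animated chest actor whose lid moves on a timeline from BeginPlay, with an Interact event that checks whether the lid is closed.
; Interacting with the lid roll at -5 degrees or above sets IsClosed, stops the timeline, spawns BP_ChestClosed and plays a slam sound.
; Below that threshold it spawns BP_ChestFalseClosed, plays another sound and resumes the timeline.
; Once closed, further interactions repeat the closed response.
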(event `Interact`
  (if (`self.isClosed`)
    (`|SpawnActorFromClass` "/Game/Lessons/Lesson3/miniProject3/BP_ChestClosed.BP_ChestClosed_C" (`KismetMathLibrary.Conv_VectorToTransform` (`self.K2_GetActorLocation`)) "Undefined" "MultiplyWithRoot" null null :!label _label)
    (`GameplayStatics.PlaySound2D` "/Game/Lessons/Lesson3/miniProject3/chest-slam-85122.chest-slam-85122" 1.0 1.0 0.0 null null)
    (bind (_direction _timeline) (`Timeline|LidRotation` :!via `Stop` :!label _label_2)
      (:`Update`
        (if (not (`self.isClosed`))
          (`SceneComponent.K2_SetRelativeRotation` (`self.ChestLid`) (`KismetMathLibrary.MakeRotator` _timeline) false false))))
    (else
      (`/Engine/EditorBlueprintResources/StandardMacros.CompareFloat` (.roll (.rotation (`SceneComponent.GetRelativeTransform` (`self.ChestLid`)))) -5.0
        (:`>`
          _)
        (:`==`
          _)
        (:`<`
          (`|SpawnActorFromClass` "/Game/Lessons/Lesson3/miniProject3/BP_ChestFalseClosed.BP_ChestFalseClosed_C" (`KismetMathLibrary.Conv_VectorToTransform` (`self.K2_GetActorLocation`)) "Undefined" "MultiplyWithRoot" null null)
          (`GameplayStatics.PlaySound2D` "/Game/Lessons/Lesson3/miniProject3/chest_SFX.chest_SFX" 1.0 1.0 0.0 null null)
          (goto _label_2)))
      (set `self.isClosed` true)
      (goto _label))))

(event `self.ReceiveBeginPlay`
  (goto _label_2))

(fn `UserConstructionScript`)