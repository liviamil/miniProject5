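; BP_mp3 is a lesson mini-project Blueprint that lets a VR player interact with chests by looking at them and pressing PrimaryAction.
; The press fires a debug-drawn Visibility line trace forward from the VR camera.
; The hit actor is cast in turn, calling Interact2 on BP_ChestMonster or Interact on BP_AnimatedCHest.
; A final BP_Test cast leads to no action, and BeginPlay, overlap and Tick are unused.
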(event `InputAction|PrimaryAction`
  (params (Key :type "Key Structure"))
  (:`Pressed`
    (bind (_location _forward_vector) (`/Game/Blueprints/Utility/VARlabsVRUtilityFunctions.Get Player VR Camera Properties`))
    (bind (_outhit _returnvalue) (`KismetSystemLibrary.LineTraceSingle` :`Start` _location :`End` (+ _location (* _forward_vector (`KismetMathLibrary.Conv_DoubleToVector` 10000.0))) :`TraceChannel` "TraceTypeQuery1" :`DrawDebugType` "ForDuration" :`DrawTime` 2.0))
    (bind (_bblockinghit _binitialoverlap _time _distance _location_2 _impactpoint _normal _impactnormal _physmat _hitactor) (`GameplayStatics.BreakHitResult` _outhit))
    (bind _asbp_chest_monster (cast `/Game/Lessons/Lesson3/miniProject3/BP_ChestMonster` _hitactor)
      (:`then`
        (`/Game/Lessons/Lesson3/miniProject3/BP_ChestMonster.Interact2` _asbp_chest_monster))
      (:`CastFailed`
        (if _returnvalue
          (bind _asbp_animated_chest (cast `/Game/Lessons/Lesson3/miniProject3/BP_AnimatedCHest` _hitactor)
            (:`then`
              (`/Game/Lessons/Lesson3/miniProject3/BP_AnimatedCHest.Interact` _asbp_animated_chest))
            (:`CastFailed`
              (cast `/Game/Lessons/Lesson3/miniProject3/BP_Test` _hitactor))))))))

(fn `UserConstructionScript`)